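; Actor component that shows circular on-screen damage indicators pointing toward where its owner was hit from.
; DmgTaken spawns a UI_DamageIndicator widget, styles it through CustomSettings, and rotates it by the yaw between owner forward and damage origin.
; In Dynamic mode indicators are stored and re-angled every Tick until RemoveIndicator drops them.
; NearDamage builds a non-directional variant, but DmgTaken's distance check for it is disconnected.
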(event `self.ReceiveTick`
  (params (DeltaSeconds :type "Float (single-precision)"))
  ;[1 1 1] If dynamic is true, rotate all indicators every frame
  (if (`self.Dynamic`)
    (for _array_element (`self.PointDamageIndicators`)
      (`self.CalculateAngle` (`/Game/CircleDamageIndicator/Blueprints/UI/UI_DamageIndicator.FromLocation` _array_element) _array_element))))

(fn `CalculateAngle`
  (params (FromLocation :type "Vector Structure") (Indicator :type "/Game/CircleDamageIndicator/Blueprints/UI/UI_DamageIndicator Object Reference"))
  (bind _returnvalue (`self.GetOwner`))
  (`Widget.SetRenderAngle` (`/Game/CircleDamageIndicator/Blueprints/UI/UI_DamageIndicator.Indicator` Indicator) (- (.yaw (`KismetMathLibrary.Conv_VectorToRotator` (`KismetMathLibrary.Normal` (* (`KismetMathLibrary.GetDirectionUnitVector` FromLocation (`Actor.K2_GetActorLocation` _returnvalue)) (-1.0 -1.0 0.0))))) (.yaw (`KismetMathLibrary.Conv_VectorToRotator` (`KismetMathLibrary.Normal` (`Actor.GetActorForwardVector` _returnvalue)))))) ; Rotate him
)

(fn `CustomSettings`
  (params (IndicatorIn :type "/Game/CircleDamageIndicator/Blueprints/UI/UI_DamageIndicator Object Reference") (PointDamage :type Boolean))
  (returns (Indicator :type "/Game/CircleDamageIndicator/Blueprints/UI/UI_DamageIndicator Object Reference"))
  (bind _indicatorimage (`/Game/CircleDamageIndicator/Blueprints/UI/UI_DamageIndicator.IndicatorImage` IndicatorIn))
  (bind _neardamageindicatorimage (`/Game/CircleDamageIndicator/Blueprints/UI/UI_DamageIndicator.NearDamageIndicatorImage` IndicatorIn))
  (bind _indicatorimage_2 (`/Game/CircleDamageIndicator/Blueprints/UI/UI_DamageIndicator.IndicatorImage` IndicatorIn))
  (bind _uiscale (`self.UIScale`))
  (bind _indicator (`/Game/CircleDamageIndicator/Blueprints/UI/UI_DamageIndicator.Indicator` IndicatorIn))
  (bind _neardamageindicator (`/Game/CircleDamageIndicator/Blueprints/UI/UI_DamageIndicator.NearDamageIndicator` IndicatorIn))
  (bind _screenoffset (`self.ScreenOffset`))
  (bind _returnvalue (`KismetMathLibrary.MakeVector2D` _uiscale _uiscale))
  ;[1 1 1] Get damage type
  (if PointDamage
    (`Widget.SetVisibility` (`/Game/CircleDamageIndicator/Blueprints/UI/UI_DamageIndicator.NearDamageIndicator` IndicatorIn) "Hidden")
    ;[1 1 1] Create Widget with parameters
    (`UserWidget.AddToViewport` IndicatorIn 0)
    (`Image.SetColorAndOpacity` _indicatorimage (`self.Color`))
    (`Image.SetBrush` _indicatorimage (`self.SetImage` _indicatorimage (`self.PointIndicator`)))
    (set `/Game/CircleDamageIndicator/Blueprints/UI/UI_DamageIndicator.PointDamage` true IndicatorIn)
    (else
      (`Widget.SetVisibility` (`/Game/CircleDamageIndicator/Blueprints/UI/UI_DamageIndicator.Indicator` IndicatorIn) "Hidden")
      ;[1 1 1] Create Widget with parameters
      (`UserWidget.AddToViewport` IndicatorIn 0)
      (`Image.SetColorAndOpacity` _neardamageindicatorimage (`self.Color`))
      (`Image.SetBrush` _neardamageindicatorimage (`self.SetImage` _neardamageindicatorimage (`self.NearIndicator`)))
      (set `/Game/CircleDamageIndicator/Blueprints/UI/UI_DamageIndicator.PointDamage` false IndicatorIn)))
  ;[1 1 1] Indicator scale
  (`Widget.SetRenderScale` _indicator _returnvalue)
  (`Widget.SetRenderScale` _neardamageindicator _returnvalue)
  ;[1 1 1] Screen Offset
  (`Widget.SetRenderTranslation` _indicator _screenoffset)
  (`Widget.SetRenderTranslation` _neardamageindicator _screenoffset)
  ;[1 1 1] Indicator Sprite Offset
  (`CanvasPanelSlot.SetPosition` (`WidgetLayoutLibrary.SlotAsCanvasSlot` _indicatorimage_2) (`self.IndicatorSpriteOffset`))
  ;[1 1 1] Indicator and near indicator size
  (`CanvasPanelSlot.SetSize` (`WidgetLayoutLibrary.SlotAsCanvasSlot` _indicatorimage_2) (`self.IndicatorSpriteSize`))
  (`CanvasPanelSlot.SetSize` (`WidgetLayoutLibrary.SlotAsCanvasSlot` (`/Game/CircleDamageIndicator/Blueprints/UI/UI_DamageIndicator.NearDamageIndicatorImage` IndicatorIn)) (`self.NearIndicatorSpriteSize`))
  ;[1 1 1] Set at what speed the indicator disappears
  (set `/Game/CircleDamageIndicator/Blueprints/UI/UI_DamageIndicator.DisappearanceSpeed` (`self.DisappearanceSpeed`) IndicatorIn)
  (return IndicatorIn))

(fn `DmgTaken`
  (params (FromLocation :type "Vector Structure"))
  ;[1 1 1] Create widget and apply settings from variables
  (bind _returnvalue (`|CreateWidget` "/Game/CircleDamageIndicator/Blueprints/UI/UI_DamageIndicator.UI_DamageIndicator_C"))
  (bind _indicator (`self.CustomSettings` _returnvalue true))
  (`self.CalculateAngle` FromLocation _indicator) ; Get angle for ui element
  ;[1 1 1] Add indicators to array
  (if (`self.Dynamic`)
    (`KismetArrayLibrary.Array_Add` (`self.PointDamageIndicators`) _indicator)
    (set `/Game/CircleDamageIndicator/Blueprints/UI/UI_DamageIndicator.FromLocation` FromLocation _indicator))
  ;[1 1 1] Add link to player actor to UI indicator
  (set `/Game/CircleDamageIndicator/Blueprints/UI/UI_DamageIndicator.FromActor` (`self.GetOwner`) _indicator))

(fn `NearDamage`
  (returns (Indicator :type "/Game/CircleDamageIndicator/Blueprints/UI/UI_DamageIndicator Object Reference"))
  ;[1 1 1] Creating near damage indicator
  (bind _returnvalue (`|CreateWidget` "/Game/CircleDamageIndicator/Blueprints/UI/UI_DamageIndicator.UI_DamageIndicator_C")) ; Create widget
  (bind _indicator (`self.CustomSettings` _returnvalue)) ; Apply settings from variables
  (return _indicator))

(fn `RemoveIndicator`
  (params (Indicator :type "/Game/CircleDamageIndicator/Blueprints/UI/UI_DamageIndicator Object Reference"))
  ;[1 1 1] Remove indicator from array
  (`KismetArrayLibrary.Array_RemoveItem` (`self.PointDamageIndicators`) Indicator))