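; Base scattershot weapon whose Shoot event fires a multi-pellet burst, with animation, muzzle effects, sound and recoil-scaled camera shake, and stops the player running if ammo remains.
; Each random or fixed bullet iteration line-traces once per RaycastPositions child along a scattered direction, with persistent debug drawing left on.
; Hits spawn surface-specific particles, decals and sounds, identify character bones, apply point damage, and either push physics bodies or send tagged components' actors the bullet direction.
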(event `self.Shoot`
  (bind (_start _end) (`self.ScatterBulletDirection`))
  (bind _recoil_min (`self.Recoil_Min`))
  (bind _player (`self.Player`))
  (bind (_returnvalue_location _returnvalue_rotation) (`KismetMathLibrary.BreakTransform` (`SceneComponent.GetSocketTransform` (`self.ObjectMesh`) "Socket_Muzzle" "RTS_World")))
  (if (and (!= (`self.Ammo_InClip`) 0) (`/Game/Interaction/Blueprints/Pawn/Player/Character_Pawn_FPS.IsRun` (`self.Player`)))
    (`/Game/Interaction/Blueprints/Pawn/Player/Character_Pawn_FPS.SetRun` _player false (`/Game/Interaction/Blueprints/Pawn/Player/Character_Pawn_FPS.WalkSpeed` _player)))
  (`SkeletalMeshComponent.PlayAnimation` (`self.ObjectMesh`) (select `bool` (== (`self.Ammo_InClip`) 0) :`false` (`self.Animation Shoot`) :`true` (`self.Animation Empty`) :!type "AnimationAsset Object Reference") false)
  (`PlayerCameraManager.PlayCameraShake` :`self` (`PlayerController.PlayerCameraManager` (`GameplayStatics.GetPlayerController` (`/Game/Interaction/Blueprints/Pawn/Player/Character_Pawn_FPS.PlayerID` (`self.Player`)))) :`ShakeClass` (`self.CameraShakeClass`) :`Scale` (`KismetMathLibrary.FClamp` (+ (`self.DegreesCurrent`) _recoil_min) _recoil_min (`self.Recoil_Max`)))
  (`GameplayStatics.SpawnEmitterAtLocation` (`self.MuzzleParticle`) _returnvalue_location _returnvalue_rotation)
  (`GameplayStatics.PlaySoundAtLocation` (`self.ShotSound`) _returnvalue_location (struct) 1.0 1.0 0.0 null null null)
  (if (`self.RandomNumBullets`)
    (for _ (range (`self.Bullet_Min`) (+ (`KismetMathLibrary.RandomIntegerInRange` (`self.Bullet_Min`) (`self.Bullet_Max`)) 1))
      (for _array_element (`SceneComponent.GetChildrenComponents` (`self.RaycastPositions`) false) :!label _label
        (bind _outhit (`KismetSystemLibrary.LineTraceSingleForObjects` _start _end (`|MakeArray` "ObjectTypeQuery1" "ObjectTypeQuery2" "ObjectTypeQuery4" "ObjectTypeQuery5" "ObjectTypeQuery7" "ObjectTypeQuery9" "ObjectTypeQuery6" :!type "EObjectTypeQuery Enum") true (`|MakeArray` (`self.Player`) :!type "Actor Object Reference") "Persistent"))
        (bind (_bblockinghit _binitialoverlap _time _distance _location _impactpoint _normal _impactnormal _physmat _hitactor _hitcomponent _hitbonename _hititem _faceindex _tracestart _traceend) (`GameplayStatics.BreakHitResult` _outhit))
        (if (!= self _hitactor)
          (`self.SpreadingDecrease`)
          (`/Engine/EditorBlueprintResources/StandardMacros.IsValid` _hitactor
            (:`Is Valid`
              (bind (_particle _decal _decalsize _decalrotation _soundhit) (`self.SelectSurfaceEffects` (`PhysicalMaterial.SurfaceType` _physmat) (`KismetMathLibrary.Conv_VectorToRotator` _normal)))
              (bind (_returnvalue_roll _returnvalue_pitch _returnvalue_yaw) (`KismetMathLibrary.BreakRotator` (`KismetMathLibrary.Conv_VectorToRotator` _normal)))
              (`GameplayStatics.SpawnEmitterAtLocation` _particle _location (`KismetMathLibrary.MakeRotator` _returnvalue_roll (+ _returnvalue_pitch -90.0) _returnvalue_yaw))
              (`GameplayStatics.SpawnDecalAttached` _decal _decalsize _hitcomponent _hitbonename _impactpoint _decalrotation "KeepWorldPosition" 40.0)
              (bind _ascharacter_pawn_fps (cast `/Game/Interaction/Blueprints/Pawn/Player/Character_Pawn_FPS` _hitactor)
                (:`then`
                  (`self.IdentifyBoneHit` _hitbonename _ascharacter_pawn_fps))
                (:`CastFailed`
                  _))
              (`GameplayStatics.PlaySoundAtLocation` _soundhit _location (struct) 1.0 1.0 0.0 null null null)
              (`GameplayStatics.ApplyPointDamage` _hitactor (`self.BaseDamage`) (10.0 10.0 10.0) _outhit null (`ActorComponent.GetOwner` (`Actor.RootComponent` (`self.Player`))) (`self.DamageType`))
              (if (`ActorComponent.ComponentHasTag` _hitcomponent "CustomImpusle")
                (bind _returnvalue (`KismetMathLibrary.Normal` (- _traceend (`SceneComponent.GetSocketLocation` (`/Game/Interaction/Blueprints/Weapon/Base_Interactive_Object_Class.ObjectMesh` (`/Game/Interaction/Blueprints/Pawn/Player/Character_Pawn_FPS.CWeapon` (`self.Player`))) "Socket_Muzzle"))))
                (message `/Game/Interaction/Blueprints/Weapon/WeaponInterface.GetBulletDirection` _hitactor _returnvalue _hitbonename)
                (elif (`SceneComponent.IsSimulatingPhysics` _hitcomponent _hitbonename)
                  (`PrimitiveComponent.AddImpulse` _hitcomponent (* _returnvalue 200.0) _hitbonename true))))))))
    (else
      (for _ (range (`self.Bullet_Min`) (+ (`self.Bullet_Max`) 1))
        (goto _label)))))

(fn `UserConstructionScript`
  (`parent.UserConstructionScript`))