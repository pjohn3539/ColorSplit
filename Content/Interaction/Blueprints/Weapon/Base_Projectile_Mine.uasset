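; Base mine projectile Blueprint that detects its first valid impact and passes character bone hits to its origin weapon.
; Collider overlap filters out itself and its owner, latches HitTarget, then line-traces forward from the Sphere to find the hit.
; A valid hit spawns a normal-aligned emitter, plays sound and zeroes Speed.
; Decal, point damage and destroy nodes are unconnected; debug trace drawing and bone-name printing remain active.
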(event `self.Collider.OnComponentBeginOverlap`
  (params (OverlappedComponent :type "PrimitiveComponent Object Reference") (OtherActor :type "Actor Object Reference") (OtherComp :type "PrimitiveComponent Object Reference") (OtherBodyIndex :type Integer) (bFromSweep :type Boolean) (SweepResult :type "HitResult Structure (by ref)"))
  (bind _returnvalue (`self.GetOwner`))
  (if (and (!= (`self.GetOwner` OtherActor) _returnvalue) (!= self OtherActor) (!= _returnvalue OtherActor) (not (`self.HitTarget`)) (`|EnumInequality` (`PrimitiveComponent.GetCollisionObjectType` OverlappedComponent) "ECC_Pawn"))
    (set `self.HitTarget` true)
    (`GameplayStatics.PlaySoundAtLocation` (`self.ImpactSound`) (`self.K2_GetActorLocation`) (struct) 1.0 1.0 0.0 null null null)
    (bind _outhit (`KismetSystemLibrary.LineTraceSingleForObjects` :`Start` (`SceneComponent.K2_GetComponentLocation` (`self.Sphere`)) :`End` (+ (`SceneComponent.K2_GetComponentLocation` (`self.Sphere`)) (* (`KismetMathLibrary.GetForwardVector` (`self.K2_GetActorRotation`)) (`self.DistanceForward`))) :`ObjectTypes` (`|MakeArray` "ObjectTypeQuery1" "ObjectTypeQuery2" "ObjectTypeQuery4" "ObjectTypeQuery5" "ObjectTypeQuery7" "ObjectTypeQuery9" "ObjectTypeQuery6" :!type "EObjectTypeQuery Enum") :`bTraceComplex` true :`DrawDebugType` "Persistent"))
    (bind (_bblockinghit _binitialoverlap _time _distance _location _impactpoint _normal _impactnormal _physmat _hitactor _hitcomponent _hitbonename) (`GameplayStatics.BreakHitResult` _outhit))
    ;[1 1 1] Bullet Hit
    (if (!= self _hitactor)
      (`KismetSystemLibrary.PrintString` (`KismetStringLibrary.Conv_NameToString` _hitbonename))
      (`/Engine/EditorBlueprintResources/StandardMacros.IsValid` _hitactor
        (:`Is Valid`
          (bind (_returnvalue_roll _returnvalue_pitch _returnvalue_yaw) (`KismetMathLibrary.BreakRotator` (`KismetMathLibrary.Conv_VectorToRotator` _normal)))
          (`GameplayStatics.SpawnEmitterAtLocation` null _location (`KismetMathLibrary.MakeRotator` _returnvalue_roll (+ _returnvalue_pitch -90.0) _returnvalue_yaw))
          (bind _ascharacter_pawn_fps (cast `/Game/Interaction/Blueprints/Pawn/Player/Character_Pawn_FPS` _hitactor)
            (:`then`
              (`/Game/Interaction/Blueprints/Weapon/Weapon_Ammo_Class.IdentifyBoneHit` (`self.OriginWeapon`) _hitbonename _ascharacter_pawn_fps))
            (:`CastFailed`
              _))
          (`GameplayStatics.PlaySoundAtLocation` "/Game/Interaction/Blueprints/Commentary_Box/Assets/Audio/Blueprints_TextPop01.Blueprints_TextPop01" _location (struct) 1.0 1.0 0.0 null null null)
          (set `self.Speed` 0.0))))))

(fn `UserConstructionScript`
  (`parent.UserConstructionScript`))