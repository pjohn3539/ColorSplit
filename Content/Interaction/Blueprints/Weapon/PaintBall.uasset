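; Paintball projectile that copies damage, speed and player from its owning Base_Shooting_Weapon and drives its physics sphere forward every Tick.
; On overlapping a non-owner FPS character, it line-traces ahead, passes the hit bone to the weapon, applies point damage, plays impact effects, spawns a decal and destroys itself.
; Most other overlaps just leave a decal and destroy it.
; Debug prints and a persistent trace drawing remain active.
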(event `self.ReceiveBeginPlay`
  (bind _asbase_shooting_weapon (cast `/Game/Interaction/Blueprints/Weapon/Base_Shooting_Weapon` (`self.GetOwner`)))
  (set `self.Damage` (`/Game/Interaction/Blueprints/Weapon/Weapon_Ammo_Class.BaseDamage` _asbase_shooting_weapon))
  (set `self.Speed` (`/Game/Interaction/Blueprints/Weapon/Base_Shooting_Weapon.ProjectileSpeed` _asbase_shooting_weapon))
  (set `self.Player` (`/Game/Interaction/Blueprints/Weapon/Base_Interactive_Object_Class.Player` _asbase_shooting_weapon))
  (set `self.StoppingPower` (`/Game/Interaction/Blueprints/Weapon/Base_Weapon_Class.CurrentStoppingPower` _asbase_shooting_weapon))
  (bind _asbase_shooting_weapon_2 (cast `/Game/Interaction/Blueprints/Weapon/Base_Shooting_Weapon` (`self.GetOwner`)))
  (set `self.OriginWeapon` _asbase_shooting_weapon_2)
  (bind _asinteraction_game_mode_fps (cast `/Game/GameManagers/Interaction_GameMode_FPS` (`GameplayStatics.GetGameMode`)))
  (set `self.GameMode` _asinteraction_game_mode_fps))

(event `self.ReceiveTick`
  (params (DeltaSeconds :type "Float (single-precision)"))
  (`PrimitiveComponent.SetPhysicsLinearVelocity` (`self.Sphere`) (* (`KismetMathLibrary.GetForwardVector` (`self.K2_GetActorRotation`)) (`self.Speed`)) false "None"))

(event `self.Collider.OnComponentBeginOverlap`
  (params (OverlappedComponent :type "PrimitiveComponent Object Reference") (OtherActor :type "Actor Object Reference") (OtherComp :type "PrimitiveComponent Object Reference") (OtherBodyIndex :type Integer) (bFromSweep :type Boolean) (SweepResult :type "HitResult Structure (by ref)"))
  (`KismetSystemLibrary.PrintString` "help"))

(event `self.Sphere.OnComponentBeginOverlap`
  (params (OverlappedComponent :type "PrimitiveComponent Object Reference") (OtherActor :type "Actor Object Reference") (OtherComp :type "PrimitiveComponent Object Reference") (OtherBodyIndex :type Integer) (bFromSweep :type Boolean) (SweepResult :type "HitResult Structure (by ref)"))
  (bind _returnvalue (`KismetStringLibrary.Concat_StrStr` (`KismetStringLibrary.Concat_StrStr` (`KismetStringLibrary.Concat_StrStr` "Actor: " (`KismetSystemLibrary.GetObjectName` OverlappedComponent)) " ") (`KismetStringLibrary.Concat_StrStr` "Comp: " (`KismetSystemLibrary.GetDisplayName` OverlappedComponent))))
  (if (!= self OtherActor)
    (if (and (!= (`self.GetOwner` OtherActor) (`self.GetOwner`)) (`|EnumInequality` (`PrimitiveComponent.GetCollisionObjectType` OverlappedComponent) "ECC_Pawn"))
      (cast `/Game/Interaction/Blueprints/Pawn/Player/Character_Pawn_FPS` OtherActor
        (:`then`
          (if (and (!= (`self.GetOwner`) OtherActor) (not (`self.HitTarget`)))
            (set `self.HitTarget` true)
            (`GameplayStatics.PlaySoundAtLocation` (`self.ImpactSound`) (`self.K2_GetActorLocation`) (struct) 1.0 1.0 0.0 null null null)
            (bind _outhit (`KismetSystemLibrary.LineTraceSingleForObjects` :`Start` (`SceneComponent.K2_GetComponentLocation` (`self.Sphere`)) :`End` (+ (`SceneComponent.K2_GetComponentLocation` (`self.Sphere`)) (* (`KismetMathLibrary.GetForwardVector` (`self.K2_GetActorRotation`)) (`self.DistanceForward`))) :`ObjectTypes` (`|MakeArray` "ObjectTypeQuery1" "ObjectTypeQuery2" "ObjectTypeQuery4" "ObjectTypeQuery5" "ObjectTypeQuery7" "ObjectTypeQuery9" "ObjectTypeQuery6" :!type "EObjectTypeQuery Enum") :`bTraceComplex` true :`DrawDebugType` "Persistent"))
            (bind (_bblockinghit _binitialoverlap _time _distance _location _impactpoint _normal _impactnormal _physmat _hitactor _hitcomponent _hitbonename) (`GameplayStatics.BreakHitResult` _outhit))
            ;[1 1 1] Bullet Hit
            (if (!= self _hitactor)
              (`KismetSystemLibrary.PrintString` (`KismetStringLibrary.Conv_NameToString` _hitbonename))
              (`/Engine/EditorBlueprintResources/StandardMacros.IsValid` _hitactor
                (:`Is Valid`
                  (bind (_returnvalue_roll _returnvalue_pitch _returnvalue_yaw) (`KismetMathLibrary.BreakRotator` (`KismetMathLibrary.Conv_VectorToRotator` _normal)))
                  (`GameplayStatics.SpawnEmitterAtLocation` null _location (`KismetMathLibrary.MakeRotator` _returnvalue_roll (+ _returnvalue_pitch -90.0) _returnvalue_yaw))
                  (bind _ascharacter_pawn_fps (cast `/Game/Interaction/Blueprints/Pawn/Player/Character_Pawn_FPS` _hitactor)
                    (:`then`
                      (`/Game/Interaction/Blueprints/Weapon/Weapon_Ammo_Class.IdentifyBoneHit` (`self.OriginWeapon`) _hitbonename _ascharacter_pawn_fps false false))
                    (:`CastFailed`
                      _))
                  (`GameplayStatics.PlaySoundAtLocation` "/Game/Interaction/Blueprints/Commentary_Box/Assets/Audio/Blueprints_TextPop01.Blueprints_TextPop01" _location (struct) 1.0 1.0 0.0 null null null)
                  (`GameplayStatics.ApplyPointDamage` _hitactor (`self.Damage`) (10.0 10.0 10.0) _outhit null (`self.Player`) "/Game/Interaction/Blueprints/Weapon/BP_DamageType_handgun.BP_DamageType_handgun_C")
                  (bind _returnvalue_2 (`GameplayStatics.SpawnDecalAtLocation` "/Game/Materials/OutLineColors/Decals/GrenadeMaterial.GrenadeMaterial" (250.0 250.0 250.0) (`SceneComponent.K2_GetComponentLocation` (`self.Sphere`))))
                  (`KismetSystemLibrary.PrintString` (`KismetStringLibrary.Conv_VectorToString` (`SceneComponent.K2_GetComponentLocation` _returnvalue_2)) true true (struct :`G` 0.66 :`B` 1.0 :`A` 1.0) 60.0)
                  (`self.K2_DestroyActor`))))
            (else
              (`KismetSystemLibrary.PrintString` _returnvalue))))
        (:`CastFailed`
          (`KismetSystemLibrary.PrintString` _returnvalue)
          (`GameplayStatics.SpawnDecalAtLocation` "/Game/Materials/OutLineColors/Decals/GrenadeMaterial.GrenadeMaterial" (250.0 250.0 250.0) (`SceneComponent.K2_GetComponentLocation` (`self.Sphere`)) :!label _label)
          (`self.K2_DestroyActor`)))
      (else
        (`KismetSystemLibrary.PrintString` _returnvalue)
        (goto _label)))))

(fn `UserConstructionScript`)