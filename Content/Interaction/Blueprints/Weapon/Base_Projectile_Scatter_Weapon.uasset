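; Base weapon Blueprint for scatter guns that fire multiple projectile bullets per shot.
; Shoot cancels the player's run when CheckIfRunning passes, then plays the mesh animation, muzzle particle and sound at the muzzle socket.
; A fixed or randomized loop spawns Base_Projectile_Bullet actors at every child component of BulletSpawnPoint, so component transforms define the spread.
; The recoil camera shake is disconnected and never runs.
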(event `self.Shoot`
  (bind _player (`self.Player`))
  (bind (_returnvalue_location _returnvalue_rotation) (`KismetMathLibrary.BreakTransform` (`SceneComponent.GetSocketTransform` (`self.ObjectMesh`) "Socket_Muzzle" "RTS_World")))
  ;[1 1 1] Shoot Animation Select
  (if (`self.CheckIfRunning`)
    (`/Game/Interaction/Blueprints/Pawn/Player/Character_Pawn_FPS.SetRun` _player false (`/Game/Interaction/Blueprints/Pawn/Player/Character_Pawn_FPS.WalkSpeed` _player)))
  (`SkeletalMeshComponent.PlayAnimation` (`self.ObjectMesh`) null false)
  ;[1 1 1] Muzzle
  (`GameplayStatics.SpawnEmitterAtLocation` (`self.MuzzleParticle`) _returnvalue_location _returnvalue_rotation)
  ;[1 1 1] Shoot Sound
  (`GameplayStatics.PlaySoundAtLocation` null _returnvalue_location (struct) 1.0 1.0 0.0 null null null)
  ;[1 1 1] Bullet
  (if (`self.RandomNumBullets`)
    (for _ (range (`self.Bullet_Min`) (+ (`KismetMathLibrary.RandomIntegerInRange` (`self.Bullet_Min`) (`self.Bullet_Max`)) 1))
      (for _array_element (`SceneComponent.GetChildrenComponents` (`self.BulletSpawnPoint`) false) :!label _label
        (`|SpawnActorFromClass` "/Game/Interaction/Blueprints/Weapon/Base_Projectile_Bullet.Base_Projectile_Bullet_C" (`KismetMathLibrary.MakeTransform` (`SceneComponent.K2_GetComponentLocation` _array_element) (`SceneComponent.K2_GetComponentRotation` _array_element)) "Undefined" "OverrideRootScale" self null)))
    (else
      (for _ (range (`self.Bullet_Min`) (+ (`self.Bullet_Max`) 1))
        (goto _label)))))

(fn `UserConstructionScript`
  (`parent.UserConstructionScript`))