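; Music manager that starts the first MusicList track as a 2D sound on BeginPlay and is set up for menu and gameplay music transitions.
; Tick runs FadeIn, ramping volume by elapsed time, unless the FadeOut flag is set.
; PressPlay and ExitToMenu set transition flags, the next song index and FadeOut.
; The switch is unfinished: nothing here calls the FadeOut function or plays the next song.
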(event `self.ReceiveBeginPlay`
  (bind _returnvalue (`GameplayStatics.SpawnSound2D` (`|GetArrayItem` (`self.MusicList`)) 0.5 1.0 0.0 null))
  (set `self.MusicPlay` _returnvalue))

(event `self.ReceiveTick`
  (params (DeltaSeconds :type "Float (single-precision)"))
  (if (`self.Fade Out`)
    _
    (elif (`self.Fade In`)
      (`self.FadeIn` DeltaSeconds))))

(event `PressPlay`
  (set `self.TransitionToPlay` true)
  (set `self.NextSongIndex` 1)
  (set `self.Fade Out` true :!label _label))

(event `ExitToMenu`
  (set `self.TransitionToMainMenu` true)
  (set `self.NextSongIndex` 0)
  (goto _label))

(fn `FadeIn`
  (params (DeltaTime :type "Float (double-precision)"))
  (bind _output_get (set `self.FadedSeconds` (+ DeltaTime (`self.FadedSeconds`))))
  (if (>= _output_get (`self.SecondsToFadeIn`))
    (`AudioComponent.AdjustVolume` (`self.MusicPlay`) 0.0 1.0)
    (set `self.Fade In` false)
    (set `self.FadedSeconds` 0.0)
    (else
      (`AudioComponent.AdjustVolume` (`self.MusicPlay`) 0.1 (/ (`self.FadedSeconds`) (`self.SecondsToFadeIn`))))))

(fn `FadeOut`
  (params (DeltaTime :type "Float (double-precision)"))
  (bind _output_get (set `self.FadedSeconds` (+ DeltaTime (`self.FadedSeconds`))))
  (if (>= _output_get (`self.SecondsToFadeIn`))
    (`AudioComponent.AdjustVolume` (`self.MusicPlay`) 0.0 1.0)
    (set `self.Fade In` false)
    (set `self.FadedSeconds` 0.0)
    (else
      (`AudioComponent.AdjustVolume` (`self.MusicPlay`) 0.1 (- 0.0 (/ (`self.FadedSeconds`) (`self.SecondsToFadeIn`)))))))

(fn `UserConstructionScript`)